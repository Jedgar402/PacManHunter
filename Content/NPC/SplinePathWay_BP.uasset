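; Spline path actor in the NPC folder that moves a static mesh along a spline, starting on BeginPlay and looping from the start after a brief delay.
; A timeline alpha maps to distance along the spline, updating the mesh position and a stored Location variable.
; Pause and Continue events stop and resume the timeline.
; Sphere overlaps with NPC actors toggle an OverlappingNPC flag.
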(event `Continue`
  (bind (_direction _spline_track_) (`Timeline|Timeline_0` :!label _label)
    (:`Update`
      (bind _returnvalue (`SplineComponent.GetLocationAtDistanceAlongSpline` (`self.Spline`) (`KismetMathLibrary.Lerp` 0.0 (`SplineComponent.GetSplineLength` (`self.Spline`)) _spline_track_) "World"))
      (set `self.Location` _returnvalue)
      (`SceneComponent.K2_SetWorldLocation` (`self.StaticMesh`) _returnvalue false false))
    (:`Finished`
      (`KismetSystemLibrary.Delay` 0.2)
      (goto _label :!via `PlayFromStart`))))

(event `self.ReceiveBeginPlay`
  (goto _label))

(event `Pause`
  (goto _label :!via `Stop`))

(event `self.Sphere.OnComponentBeginOverlap`
  (params (OverlappedComponent :type "PrimitiveComponent Object Reference") (OtherActor :type "Actor Object Reference") (OtherComp :type "PrimitiveComponent Object Reference") (OtherBodyIndex :type Integer) (bFromSweep :type Boolean) (SweepResult :type "HitResult Structure (by ref)"))
  (cast `/Game/NPC/NPC` OtherActor)
  (set `self.OverlappingNPC?` true))

(event `self.Sphere.OnComponentEndOverlap`
  (params (OverlappedComponent :type "PrimitiveComponent Object Reference") (OtherActor :type "Actor Object Reference") (OtherComp :type "PrimitiveComponent Object Reference") (OtherBodyIndex :type Integer))
  (cast `/Game/NPC/NPC` OtherActor)
  (set `self.OverlappingNPC?` false))

(fn `UserConstructionScript`)